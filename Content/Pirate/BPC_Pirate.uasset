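; Pirate AI melee character that plays attack montages and drives Blackboard flags for sensing and exhaustion.
; Attack picks a random normal montage, switching to a random advanced move once the counter reaches four, then resetting it.
; Seeing a pawn briefly sets InRangeAttack; Exhaust runs a sitting pause that clears the Exhaust flag afterward.
; Attack and Exhaust return fixed durations to their caller.
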(event `NormalAttack`
  ; Normal Attack
  (switch `int` (`KismetMathLibrary.RandomIntegerInRange` 0 4)
    (:`Default`
      (`self.PlayAnimMontage` "/Game/Pirate/Animation/AM_Matelo.AM_Matelo" :!label _label))
    (:`0`
      (goto _label))
    (:`1`
      (`self.PlayAnimMontage` "/Game/Pirate/Animation/AM_Pontera.AM_Pontera"))
    (:`2`
      (`self.PlayAnimMontage` "/Game/Pirate/Animation/AM_Stable.AM_Stable"))
    (:`3`
      (`self.PlayAnimMontage` "/Game/Pirate/Animation/AM_Torch.AM_Torch")))
  (bind _result (`/Engine/EditorBlueprintResources/StandardMacros.IncrementInt` (`self.AttackTime`))
    (:`  `
      (set `self.AttackTime` _result))))

(event `Combo`
  ; Combo
  (if (>= (`self.AttackTime`) 4)
    (`self.Advantage Attack`)
    (else
      (`self.NormalAttack`))))

(event `self.PawnSensing.OnSeePawn`
  (params (Pawn :type "Pawn Object Reference"))
  ; Sensing
  (`BlackboardComponent.SetValueAsBool` (`AIBlueprintHelperLibrary.GetBlackboard` (`AIBlueprintHelperLibrary.GetAIController` self)) "InRangeAttack" true)
  (`KismetSystemLibrary.Delay` 1.6)
  (`BlackboardComponent.SetValueAsBool` (`AIBlueprintHelperLibrary.GetBlackboard` (`AIBlueprintHelperLibrary.GetAIController` self)) "InRangeAttack" false))

(event `Advantage Attack`
  ; Advantage Attack
  (switch `int` (`KismetMathLibrary.RandomIntegerInRange` 0 4)
    (:`Default`
      (`self.PlayAnimMontage` "/Game/Pirate/Animation/AM_BackToFlip.AM_BackToFlip" 3.0 :!label _label_2))
    (:`0`
      (goto _label_2))
    (:`1`
      (`self.PlayAnimMontage` "/Game/Pirate/Animation/AM_Hurricane.AM_Hurricane"))
    (:`2`
      (`self.PlayAnimMontage` "/Game/Pirate/Animation/AM_Inside_Crescent_Kick.AM_Inside_Crescent_Kick"))
    (:`3`
      (`self.PlayAnimMontage` "/Game/Pirate/Animation/AM_Kicking.AM_Kicking")))
  (set `self.AttackTime` 0))

(event `Sitting`
  ; Exhast
  (`self.PlayAnimMontage` null 2.0)
  (`KismetSystemLibrary.Delay` 4.0)
  (`BlackboardComponent.SetValueAsBool` (`AIBlueprintHelperLibrary.GetBlackboard` (`AIBlueprintHelperLibrary.GetAIController` self)) "Exhaust" false))

(fn `Attack`
  (returns (Duration :type "Float (double-precision)"))
  (`self.Combo`)
  (return 1.3))

(fn `Exhaust`
  (returns (Duration :type "Float (double-precision)"))
  (`self.Sitting`)
  (return 4.0))

(fn `UserConstructionScript`)