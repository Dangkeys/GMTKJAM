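; BPC_Stamina is a stamina component that stores a current Stamina value and exposes functions to read and change it.
; Modify adds a signed amount, clamps the result between zero and MaxStamina, and returns it.
; Decrease passes DecreaseAmount to Modify and returns the new value, while GetStamina returns the current one.
; Increase is an empty stub, and BeginPlay and Tick are unused.
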(fn `Decrease`
  (returns (Stamina :type "Float (double-precision)"))
  (`self.Modify` (`self.DecreaseAmount`))
  (return (`self.Stamina`)))

(fn `GetStamina`
  (returns (Stamina :type "Float (double-precision)"))
  (return (`self.Stamina`)))

(fn `Increase`)

(fn `Modify`
  (params (Amount :type "Float (double-precision)"))
  (returns (Output_Get :type "Float (double-precision)"))
  (bind _output_get (set `self.Stamina` (`KismetMathLibrary.FClamp` (+ (`self.Stamina`) Amount) 0.0 (`self.MaxStamina`))))
  (return _output_get))